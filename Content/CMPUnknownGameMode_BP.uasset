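; Game mode for an endless tile-based level that spawns track tiles and holds score, spawn count and spawn delay.
; Each TileVar1_BP spawns at the previous tile's attach point, raising the spawn count, or at a Y offset computed from the tile number.
; Tiles receive a shared NavMesh bounds volume pool, populated at BeginPlay.
; A bound event moves the White Mountains landscape, and helpers destroy actors by class or shorten the spawn delay.
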(event `self.ReceiveBeginPlay`
  (add `self.MoveLandscape` (delegate `EventMoveLandscape_Event`))
  (`self.PopulateBoundsVolumePool`))

(event `EventMoveLandscape_Event`
  (`KismetSystemLibrary.PrintString` "EventCalled")
  (bind _outactors (`GameplayStatics.GetAllActorsOfClass` "/Game/WhiteMountainsLandscape_BP.WhiteMountainsLandscape_BP_C"))
  (`/Game/WhiteMountainsLandscape_BP.MovingLandscape` (`KismetArrayLibrary.Array_Get` _outactors)))

(event `self.ReceiveTick`
  (params (DeltaSeconds :type "Float (single-precision)")))

(fn `DecreaseSpawnRate`
  (bind _spawndelay (`self.SpawnDelay`))
  (if (> _spawndelay 1.0)
    (set `self.SpawnDelay` (- _spawndelay 0.5))
    (else
      (set `self.SpawnDelay` _spawndelay))))

(fn `DestroyActors`
  (params (NewParam :type "Actor Class Reference"))
  (bind _outactors (`GameplayStatics.GetAllActorsOfClass` NewParam))
  (for _array_element _outactors
    (`self.K2_DestroyActor` _array_element)))

(fn `GetNormalLoaded`
  (returns (IsNormal :type Boolean))
  (return (`self.NormalLoaded`)))

(fn `GetNumberToSpawn`
  (returns (NewParam :type Integer))
  (return (`self.NumberToSpawn`)))

(fn `GetScore`
  (returns (Score :type Integer))
  (return (`self.Score`)))

(fn `GetSpawnDelay`
  (returns (SpawnDelay :type "Float (double-precision)"))
  (return (`self.SpawnDelay`)))

(fn `IncreaseScore`
  (params (NewParam :type Integer))
  (set `self.Score` (+ NewParam (`self.Score`))))

(fn `ProcessTransform`
  (returns (`Y Offset` :type "Float (double-precision)"))
  (locals (NewLocalVar_0 :type Integer :default 0))
  (bind _tilenumber (`self.TileNumber`))
  (bind _result (`/Engine/EditorBlueprintResources/StandardMacros.DecrementInt` _tilenumber)
    (:`  `
      (if (< _result 0)
        (set `self.TileNumber` 0))
      (return (`KismetMathLibrary.Conv_IntToDouble` (* _tilenumber -4096))))))

(fn `SetNormalLoaded`
  (params (NewParam :type Boolean))
  (set `self.NormalLoaded` NewParam))

(fn `Spawn Tile`
  (bind _next_tile_transform (`self.Next Tile Transform`))
  (set `self.CurrentTileTransform` _next_tile_transform)
  (bind _returnvalue (`|SpawnActorFromClass` "/Game/Dynamic/Terrain/TileVar1_BP.TileVar1_BP_C" _next_tile_transform "Undefined" "OverrideRootScale"))
  (`TileBase.SetPool` _returnvalue (`self.NavMeshBoundsVolumePool`))
  (bind _attach_transform (`/Game/Dynamic/Terrain/TileVar1_BP.GetAttachLocation` _returnvalue))
  (set `self.Next Tile Transform` (`KismetMathLibrary.MakeTransform` (.location _attach_transform) (.rotation _attach_transform)))
  (bind _result (`/Engine/EditorBlueprintResources/StandardMacros.IncrementInt` (`self.TileNumber`))
    (:`  `
      (set `self.TileNumber` _result)
      (bind _result_2 (`/Engine/EditorBlueprintResources/StandardMacros.IncrementInt` (`self.NumberToSpawn`))
        (:`  `
          (set `self.NumberToSpawn` _result_2))))))

(fn `SpawnTileOffset`
  (bind _y_offset (`self.ProcessTransform`))
  (bind _returnvalue (`|SpawnActorFromClass` "/Game/Dynamic/Terrain/TileVar1_BP.TileVar1_BP_C" (`KismetMathLibrary.MakeTransform` (`KismetMathLibrary.MakeVector` 0.0 _y_offset)) "Undefined" "OverrideRootScale"))
  (`TileBase.SetPool` _returnvalue (`self.NavMeshBoundsVolumePool`))
  (bind _attach_transform (`/Game/Dynamic/Terrain/TileVar1_BP.GetAttachLocation` _returnvalue))
  (set `self.Next Tile Transform` (`KismetMathLibrary.MakeTransform` (.location _attach_transform) (.rotation _attach_transform) (.scale _attach_transform))))

(fn `UserConstructionScript`)