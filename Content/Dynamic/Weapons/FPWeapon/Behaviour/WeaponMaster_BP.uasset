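; WeaponMaster_BP is a master weapon Blueprint that attaches to a pawn's right-hand socket, registers as its equipped weapon and fires projectiles.
; StartFire calls CameraAim, which line-traces from the muzzle toward a distant point along the owner's view aim.
; It immediately spawns an explosion effect at AimVector and launches BP_PlayerProjectile from the muzzle using control rotation.
; SetOwningPawn also sets the network owner, while StopFire is an empty stub.
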(fn `AttachToOwner`
  (bind _owningpawn (`self.OwningPawn`))
  (`/Engine/EditorBlueprintResources/StandardMacros.IsValid` _owningpawn
    (:`Is Valid`
      (`SceneComponent.K2_AttachToComponent` (`self.WeaponMesh`) (`Character.Mesh` _owningpawn) (`/Game/Dynamic/Character/Blueprints/CharacterPlayer_BP.RHand_WeaponSocket` _owningpawn) "SnapToTarget" "SnapToTarget" "KeepWorld" true)
      (set `/Game/Dynamic/Character/Blueprints/CharacterPlayer_BP.EquippedWeapon` self _owningpawn))))

(fn `CameraAim`
  (bind _muzzlelocation (`self.GetMuzzleLocation`))
  (bind _owningpawn (`self.OwningPawn`))
  (set `self.AimVector` (`KismetMathLibrary.GetForwardVector` (`Pawn.GetBaseAimRotation` _owningpawn)))
  (bind _ascharacter_player_controller (`/Game/Dynamic/Character/Blueprints/CharacterPlayer_BP.GetCastedOwner` _owningpawn))
  (bind _returnvalue (+ (`/Game/Dynamic/Character/Blueprints/CharacterPlayerController.GetViewPoint` _ascharacter_player_controller) (* (`/Game/Dynamic/Character/Blueprints/CharacterPlayerController.GetAimVector` _ascharacter_player_controller) 100000.0)))
  (bind _outhit (`KismetSystemLibrary.LineTraceSingle` _muzzlelocation _returnvalue "TraceTypeQuery1"))
  (bind (_bblockinghit _binitialoverlap _time _location) (`GameplayStatics.BreakHitResult` _outhit))
  (set `self.AimVector` (`KismetMathLibrary.SelectVector` _location (- _muzzlelocation _returnvalue) _bblockinghit))
  (return))

(fn `GetMuzzleLocation`
  (returns (MuzzleLocation :type "Vector Structure"))
  (return (`SceneComponent.GetSocketLocation` (`self.WeaponMesh`) (`self.MuzzleSocket`))))

(fn `SetOwningPawn`
  (params (OwningPawn :type "/Game/Dynamic/Character/Blueprints/CharacterPlayer_BP Object Reference"))
  ;[1 1 1] ForMultiplayer - functions as a cast to Player Character
  (if (!= OwningPawn (`self.OwningPawn`))
    (bind _output_get (set `self.OwningPawn` OwningPawn))
    ;;[1 1 1] For network
    (`self.SetOwner` _output_get)))

(fn `StartFire`
  (`self.CameraAim`)
  (`GameplayStatics.SpawnEmitterAtLocation` "/Game/StarterContent/Particles/P_Explosion.P_Explosion" (`self.AimVector`))
  (`|SpawnActorFromClass` "/Game/Dynamic/Weapons/FPWeapon/Behaviour/BP_PlayerProjectile.BP_PlayerProjectile_C" (`KismetMathLibrary.MakeTransform` (`self.GetMuzzleLocation`) (`Pawn.GetControlRotation` (`self.OwningPawn`))) "AlwaysSpawn" "OverrideRootScale"))

(fn `StopFire`)

(fn `UserConstructionScript`)