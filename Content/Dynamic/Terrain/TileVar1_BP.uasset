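; Terrain tile variant for a chained level, spawning grass and containers on BeginPlay and staging an enemy encounter.
; The player entering LockingVolume slides the doors open via a timeline and has the game mode spawn the next tile once.
; The StartGame trigger blocks further door opening and spawns heavy mutants at randomized delays, using game mode count and delay.
; The GarbageCollection trigger destroys the tile; lock and unlock functions are empty.
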(event `self.ReceiveBeginPlay`
  (`GrassComponent.SpawnGrass` (`self.GrassVar1`) 3000)
  (`GrassComponent.SpawnGrass` (`self.GrassVar2`) 500)
  (`self.PlaceActors` "/Game/Dynamic/Terrain/BP_Container.BP_Container_C" (make `ItemVariables` 1 5 500.0 1.0 1.0 true)))

(event `self.LockingVolume.OnComponentBeginOverlap`
  (params (OverlappedComponent :type "PrimitiveComponent Object Reference") (OtherActor :type "Actor Object Reference") (OtherComp :type "PrimitiveComponent Object Reference") (OtherBodyIndex :type Integer) (bFromSweep :type Boolean) (SweepResult :type "HitResult Structure (by ref)"))
  (`self.CanOpenDoor` OtherActor)
  (`|ExecutionSequence`
    (:`then_0`
      (if (`self.HaveNotSpawnedNewTile`)
        (bind _ascmpunknown_game_mode_bp (cast `/Game/CMPUnknownGameMode_BP` (`GameplayStatics.GetGameMode`)))
        (`/Game/CMPUnknownGameMode_BP.Spawn Tile` _ascmpunknown_game_mode_bp)
        (set `self.HaveNotSpawnedNewTile` false)))
    (:`then_1`
      (bind (_direction _doorposition) (`Timeline|Timeline_0` :!label _label)
        (:`Update`
          (`self.SetLeftDoor` _doorposition)
          (`self.SetRightDoor` _doorposition))))))

(event `self.LockingVolume.OnComponentEndOverlap`
  (params (OverlappedComponent :type "PrimitiveComponent Object Reference") (OtherActor :type "Actor Object Reference") (OtherComp :type "PrimitiveComponent Object Reference") (OtherBodyIndex :type Integer))
  (`self.CanOpenDoor` OtherActor)
  (goto _label :!via `Reverse`))

(event `self.GarbageCollection.OnComponentBeginOverlap`
  (params (OverlappedComponent :type "PrimitiveComponent Object Reference") (OtherActor :type "Actor Object Reference") (OtherComp :type "PrimitiveComponent Object Reference") (OtherBodyIndex :type Integer) (bFromSweep :type Boolean) (SweepResult :type "HitResult Structure (by ref)"))
  (`self.IsPlayerActor` OtherActor)
  (`self.K2_DestroyActor` self))

(event `self.StartGame.OnComponentBeginOverlap`
  (params (OverlappedComponent :type "PrimitiveComponent Object Reference") (OtherActor :type "Actor Object Reference") (OtherComp :type "PrimitiveComponent Object Reference") (OtherBodyIndex :type Integer) (bFromSweep :type Boolean) (SweepResult :type "HitResult Structure (by ref)"))
  (if (`self.TileHasNotLocked`)
    (`self.IsPlayerActor` OtherActor)
    (set `self.TileHasNotLocked` false)
    (set `self.IsFighting` true)
    (bind _ascmpunknown_game_mode_bp (cast `/Game/CMPUnknownGameMode_BP` (`GameplayStatics.GetGameMode`)))
    (bind _newparam (`/Game/CMPUnknownGameMode_BP.GetNumberToSpawn` _ascmpunknown_game_mode_bp))
    (bind _newparam_2 (`/Game/CMPUnknownGameMode_BP.GetSpawnDelay` _ascmpunknown_game_mode_bp))
    (`self.ForLoopWithDelay` 0 _newparam _newparam_2
      (:`Loop Body`
        (`self.PlaceAI` "/Game/Dynamic/Character/Blueprints/Mutant_Heavy_U1_BP.Mutant_Heavy_U1_BP_C" (make `aiVariables` 100 1.0 1.0 100 false))))))

(fn `CanDoorsMove`
  (params (Actor :type "Object Object Reference"))
  (`self.IsPlayerActor` Actor)
  (if (and (`self.IsFighting`) (`self.TileHasNotLocked`))
    _))

(fn `GetAttachLocation`
  (returns (`Attach Transform` :type "Transform Structure"))
  (return (`SceneComponent.K2_GetComponentToWorld` (`self.Arrow`))))

(fn `LockLevel`)

(fn `SetLeftDoor`
  (params (Alpha :type "Float (double-precision)"))
  (`SceneComponent.K2_SetRelativeLocation` (`self.DoorLeft`) (`KismetMathLibrary.VLerp` (`self.LeftDoorClosed`) (`self.LeftDoorOpen`) Alpha) false false))

(fn `SetRightDoor`
  (params (Alpha :type "Float (double-precision)"))
  (`SceneComponent.K2_SetRelativeLocation` (`self.DoorRight`) (`KismetMathLibrary.VLerp` (`self.RightDoorClosed`) (`self.RightDoorOpen`) Alpha) false false))

(fn `UnlockLevel`)

(fn `UserConstructionScript`)