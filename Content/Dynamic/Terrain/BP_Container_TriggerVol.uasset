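; BP_Container_TriggerVol is a trigger volume meant to swap streamed maps when the player pawn enters it, marked by its comment as deprecated and not working.
; On overlap it reads the normal-loaded flag from CMPUnknownGameMode_BP to choose between NormalMap and AlternateMap.
; It starts a non-blocking load of the other map, calls DestroyActors on the game mode, unloads the current map and flips the flag.
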(event `self.TriggerVolume.OnComponentBeginOverlap`
  (params (OverlappedComponent :type "PrimitiveComponent Object Reference") (OtherActor :type "Actor Object Reference") (OtherComp :type "PrimitiveComponent Object Reference") (OtherBodyIndex :type Integer) (bFromSweep :type Boolean) (SweepResult :type "HitResult Structure (by ref)"))
  ;[1 1 1] Depreceated - does not work
  (if (== OtherActor (`GameplayStatics.GetPlayerPawn` 0))
    (bind _ascmpunknown_game_mode_bp (cast `/Game/CMPUnknownGameMode_BP` (`GameplayStatics.GetGameMode`)))
    (bind _isnormal (`/Game/CMPUnknownGameMode_BP.GetNormalLoaded` _ascmpunknown_game_mode_bp))
    (if _isnormal
      (`GameplayStatics.LoadStreamLevel` "AlternateMap" true)
      (`/Game/CMPUnknownGameMode_BP.DestroyActors` _ascmpunknown_game_mode_bp null)
      (`GameplayStatics.UnloadStreamLevel` (`self.NormalMap`))
      (`/Game/CMPUnknownGameMode_BP.SetNormalLoaded` _ascmpunknown_game_mode_bp false)
      (else
        (`GameplayStatics.LoadStreamLevel` "NormalMap" true)
        (`/Game/CMPUnknownGameMode_BP.DestroyActors` _ascmpunknown_game_mode_bp null)
        (`GameplayStatics.UnloadStreamLevel` (`self.AlternateMap`))
        (`/Game/CMPUnknownGameMode_BP.SetNormalLoaded` _ascmpunknown_game_mode_bp true)))))

(fn `UserConstructionScript`)