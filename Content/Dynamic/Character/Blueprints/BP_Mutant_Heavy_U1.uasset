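; Heavy mutant AI enemy character that damages the player on contact.
; On begin play it enables sprinting, sets walk speed and binds its death event.
; While the player pawn overlaps the PlayerDealDamage component, a delayed while-loop macro applies damage every half second.
; Death disables that component's collision, and the loop also disables mesh collision if it finds the mutant dead.
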(event `self.ReceiveBeginPlay`
  (set `self.Sprint` true)
  (set `CharacterMovementComponent.MaxWalkSpeed` 420.0 (`self.CharacterMovement`))
  (add `self.OnDeath` (delegate `OnDeathAIEvent`)))

(event `OnDeathAIEvent`
  (`PrimitiveComponent.SetCollisionEnabled` (`self.PlayerDealDamage`) "NoCollision"))

(event `self.PlayerDealDamage.OnComponentBeginOverlap`
  (params (OverlappedComponent :type "PrimitiveComponent Object Reference") (OtherActor :type "Actor Object Reference") (OtherComp :type "PrimitiveComponent Object Reference") (OtherBodyIndex :type Integer) (bFromSweep :type Boolean) (SweepResult :type "HitResult Structure (by ref)"))
  (bind _ascharacter_player_bp (cast `/Game/Dynamic/Character/Blueprints/CharacterPlayer_BP` (`GameplayStatics.GetPlayerPawn` 0)))
  (if (== _ascharacter_player_bp OtherActor)
    (set `self.DoingDamage` true)
    (`self.WhileLoopWithDelay` (`self.DoingDamage`)
      (:`LoopBody`
        (if (`self.IsDead`)
          (`PrimitiveComponent.SetCollisionEnabled` (`self.PlayerDealDamage`) "NoCollision")
          (`PrimitiveComponent.SetCollisionEnabled` (`self.Mesh`) "NoCollision")
          (else
            (`KismetSystemLibrary.PrintString` "applying damage")
            (`GameplayStatics.ApplyDamage` OtherActor 10.0)))))))

(event `self.PlayerDealDamage.OnComponentEndOverlap`
  (params (OverlappedComponent :type "PrimitiveComponent Object Reference") (OtherActor :type "Actor Object Reference") (OtherComp :type "PrimitiveComponent Object Reference") (OtherBodyIndex :type Integer))
  (set `self.DoingDamage` false))

(fn `UserConstructionScript`
  (`parent.UserConstructionScript`))