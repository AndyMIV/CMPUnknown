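; White Mountains landscape actor that shifts its position by the offset between the game mode's current and next tile transforms.
; On BeginPlay it binds to the MovingLandscape dispatcher; each call plays the LandscapeMoving timeline, lerping from the captured location by that offset.
; A separate MoveLandscape function, not called within this Blueprint, applies the same offset instantly and prints a debug message.
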(event `self.ReceiveBeginPlay`
  (add `self.MovingLandscape` (delegate `MovingLandscape_Event`)))

(event `MovingLandscape_Event`
  (bind _pastlocation (`self.PastLocation`))
  (set `self.PastLocation` (`self.K2_GetActorLocation`))
  (bind _ascmpunknown_game_mode_bp (cast `/Game/CMPUnknownGameMode_BP` (`GameplayStatics.GetGameMode`)))
  (bind (_direction _landscape) (`Timeline|LandscapeMoving` :!via `PlayFromStart`)
    (:`Update`
      (bind _next_tile_transform_location (`KismetMathLibrary.BreakTransform` (`/Game/CMPUnknownGameMode_BP.Next Tile Transform` _ascmpunknown_game_mode_bp)))
      (bind _currenttiletransform_location (`KismetMathLibrary.BreakTransform` (`/Game/CMPUnknownGameMode_BP.CurrentTileTransform` _ascmpunknown_game_mode_bp)))
      (`self.K2_SetActorLocation` (`KismetMathLibrary.VLerp` _pastlocation (+ (- _next_tile_transform_location _currenttiletransform_location) _pastlocation) _landscape)))))

(fn `MoveLandscape`
  (bind _returnvalue (`self.K2_GetActorLocation`))
  (bind _ascmpunknown_game_mode_bp (cast `/Game/CMPUnknownGameMode_BP` (`GameplayStatics.GetGameMode`)))
  (bind _next_tile_transform_location (`KismetMathLibrary.BreakTransform` (`/Game/CMPUnknownGameMode_BP.Next Tile Transform` _ascmpunknown_game_mode_bp)))
  (bind _currenttiletransform_location (`KismetMathLibrary.BreakTransform` (`/Game/CMPUnknownGameMode_BP.CurrentTileTransform` _ascmpunknown_game_mode_bp)))
  (`self.K2_SetActorLocation` (`KismetMathLibrary.VLerp` _returnvalue (+ (- _next_tile_transform_location _currenttiletransform_location) _returnvalue) 1.0))
  (`KismetSystemLibrary.PrintString` "Moving Landscape"))

(fn `UserConstructionScript`)